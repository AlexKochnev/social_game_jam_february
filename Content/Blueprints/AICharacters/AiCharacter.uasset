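; AI character that patrols and tracks the third-person player as an enemy.
; On BeginPlay it finds the first MyAiController in the level via GetActorOfClass, rather than its possessing controller, fills health and passes it the patrol points.
; A sphere overlap sets the player as Enemy, and leaving clears it after a delay without rechecking for re-entry.
; The Attack function is an empty stub.
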(event `self.ReceiveBeginPlay`
  (`|ExecutionSequence`
    (:`then_0`
      (bind _returnvalue (`GameplayStatics.GetActorOfClass` (`self.AIControllerClass`)))
      (bind _asmy_ai_controller (cast `/Game/Blueprints/AICharacters/MyAiController` _returnvalue)
        (:`then`
          (set `self.AiController` _asmy_ai_controller))
        (:`CastFailed`
          (`KismetSystemLibrary.PrintString` "Cast failed: \"Cant Cast to AI_controller in AiCharacter\"" true true (struct :`R` 1.0 :`A` 1.0) 5.0))))
    (:`then_1`
      (set `self.Current Health` (`self.MaxHealth`)))
    (:`then_2`
      (set `/Game/Blueprints/AICharacters/MyAiController.PatrolPoints` (`self.Patrol Points`) (`self.AiController`)))))

(event `self.Sphere.OnComponentBeginOverlap`
  (params (OverlappedComponent :type "PrimitiveComponent Object Reference") (OtherActor :type "Actor Object Reference") (OtherComp :type "PrimitiveComponent Object Reference") (OtherBodyIndex :type Integer) (bFromSweep :type Boolean) (SweepResult :type "HitResult Structure (by ref)"))
  ;[1 1 1] Find enemy
  (cast `/Game/Blueprints/AICharacters/AiCharacter` OtherActor
    (:`CastFailed`
      (bind _asbp_third_person_character (cast `/Game/ThirdPerson/Blueprints/BP_ThirdPersonCharacter` OtherActor))
      (set `self.Enemy` _asbp_third_person_character)
      (set `self.Have Enemy` true))))

(event `self.Sphere.OnComponentEndOverlap`
  (params (OverlappedComponent :type "PrimitiveComponent Object Reference") (OtherActor :type "Actor Object Reference") (OtherComp :type "PrimitiveComponent Object Reference") (OtherBodyIndex :type Integer))
  ;[1 1 1] Find enemy
  (if (== OtherActor (`self.Enemy`))
    (`KismetSystemLibrary.Delay` 5.0)
    (set `self.Have Enemy` false)
    (set `self.Enemy` null)))

(fn `Attack`)

(fn `UserConstructionScript`)