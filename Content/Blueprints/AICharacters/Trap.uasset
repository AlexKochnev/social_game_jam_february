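; Trap is an AI character Blueprint for a stationary enemy that attacks without moving.
; BeginPlay runs the parent setup, then zeroes walk and swim speeds to hold it in place.
; Every Tick calls Attack while HaveEnemy is set and Enemy is valid, with target detection and the attack itself defined outside these graphs.
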(event `self.ReceiveBeginPlay`
  (`parent.ReceiveBeginPlay`)
  (set `self.MaxSwimSpeed` 0.0)
  (set `self.MaxWalkSpeed` 0.0))

(event `self.ReceiveTick`
  (params (DeltaSeconds :type "Float (single-precision)"))
  (if (`self.Have Enemy`)
    (`/Engine/EditorBlueprintResources/StandardMacros.IsValid` (`self.Enemy`)
      (:`Is Valid`
        (`self.Attack`)))))

(fn `UserConstructionScript`
  (`parent.UserConstructionScript`))