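; AI controller for an AiCharacter that patrols tagged waypoints and chases and attacks its enemy.
; DoPatrol cycles through PatrolPoints, resolving each tag by scanning all world actors and moving there with AIMoveTo.
; While HaveEnemy is set, Tick and the patrol move trigger GoToEnemy, which moves within damage radius and calls Attack.
; Patrol and chase re-enter each other through short delays, forming a loop without a behavior tree.
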(event `self.ReceiveBeginPlay`
  (bind _asai_character (cast `/Game/Blueprints/AICharacters/AiCharacter` (`self.K2_GetPawn`))
    (:`then`
      (set `self.AICharacter` _asai_character)
      (`self.DoPatrol`))
    (:`CastFailed`
      (`KismetSystemLibrary.PrintString` "Cast failed: \"Cant Cast to Ai_character in Ai_Controller\"" true true (struct :`R` 1.0 :`A` 1.0) 5.0))))

(event `GoToEnemy`
  (bind _aicharacter (`self.AICharacter`))
  (bind _enemy (`/Game/Blueprints/AICharacters/AiCharacter.Enemy` _aicharacter))
  ;[1 1 1] Patrol
  (`/Engine/EditorBlueprintResources/StandardMacros.IsValid` _enemy :!label _label
    (:`Is Valid`
      (`|AIMoveTo` _aicharacter (0.0 0.0 0.0) _enemy (`self.RadiusToDoDamage`)
        (:`then`
          (`KismetSystemLibrary.Delay` 1.0)
          (`self.DoPatrol` :!label _label_2))
        (:`OnSuccess`
          (`KismetSystemLibrary.Delay` 0.5)
          (`/Game/Blueprints/AICharacters/AiCharacter.Attack` (`self.AICharacter`)))))
    (:`Is Not Valid`
      (`KismetSystemLibrary.Delay` 0.1 :!label _label_3)
      (goto _label_2))))

(event `DoPatrol`
  (bind _patrolpoints (`self.PatrolPoints`))
  (bind _patrolcounter (`self.PatrolCounter`))
  ;[1 1 1] Patrol
  (if (not (< _patrolcounter (`KismetArrayLibrary.Array_Length` _patrolpoints)))
    (set `self.PatrolCounter` 0))
  (bind _target (`self.FindObjectByTag` (`|GetArrayItem` _patrolpoints _patrolcounter)))
  (`|AIMoveTo` (`self.AICharacter`) (0.0 0.0 0.0) _target 10.0
    (:`then`
      (if (`/Game/Blueprints/AICharacters/AiCharacter.Have Enemy` (`self.AICharacter`))
        (goto _label)))
    (:`OnSuccess`
      (`/Engine/EditorBlueprintResources/StandardMacros.IncrementInt` (`self.PatrolCounter`)
        (:`  `
          (goto _label_3))))))

(event `self.ReceiveTick`
  (params (DeltaSeconds :type "Float (single-precision)"))
  (if (`/Game/Blueprints/AICharacters/AiCharacter.Have Enemy` (`self.AICharacter`))
    (`self.GoToEnemy`)))

(fn `FindObjectByTag`
  (params (Tag :type Name))
  (returns (Target :type "Actor Object Reference"))
  (locals (TargetObject :type "Actor Object Reference"))
  (bind _outactors (`GameplayStatics.GetAllActorsOfClass` "/Script/Engine.Actor"))
  (for _array_element _outactors
    (if (`self.ActorHasTag` _array_element Tag)
      (set `local.TargetObject` _array_element)
      (break)))
  (return (`local.TargetObject`)))

(fn `UserConstructionScript`)