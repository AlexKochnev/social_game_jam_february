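; Medkit is an interactable Blueprint that gradually restores the player's health while interaction is active.
; Interact and StopInteract call their parent versions and toggle a restore flag read on Tick.
; Tick adds health at a delta-time-scaled rate while below max, draining a finite restore pool and clearing the flag once it is empty.
; The target is always player character 0, cached on BeginPlay as BP_ThirdPersonCharacter.
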(event `self.ReceiveTick`
  (params (DeltaSeconds :type "Float (single-precision)"))
  (bind _maxrestore (`self.MaxRestore`))
  (bind _interacteperson (`self.InteractePerson`))
  (bind _current_health (`/Game/ThirdPerson/Blueprints/BP_ThirdPersonCharacter.Current Health` _interacteperson))
  (if (`self.Dorestore`)
    (if (< _current_health (`/Game/ThirdPerson/Blueprints/BP_ThirdPersonCharacter.MaxHealth` _interacteperson))
      (if (not (<= _maxrestore 0.0))
        (set `/Game/ThirdPerson/Blueprints/BP_ThirdPersonCharacter.Current Health` (+ _current_health (* (`self.RestorePerTick`) DeltaSeconds)) _interacteperson)
        (set `self.MaxRestore` (- _maxrestore (* (`self.RestorePerTick`) DeltaSeconds)))
        (else
          (set `self.Dorestore` false))))))

(event `self.ReceiveBeginPlay`
  (bind _asbp_third_person_character (cast `/Game/ThirdPerson/Blueprints/BP_ThirdPersonCharacter` (`GameplayStatics.GetPlayerCharacter` 0)))
  (set `self.InteractePerson` _asbp_third_person_character))

(fn `interact`
  (`parent.interact`)
  (set `self.Dorestore` true))

(fn `StopInteract`
  (`parent.StopInteract`)
  (set `self.Dorestore` false))

(fn `UserConstructionScript`)