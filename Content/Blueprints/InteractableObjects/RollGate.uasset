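; RollGate is an interactable two-panel gate that opens on interaction and closes when something overlaps one of two trigger boxes.
; Open and Close instantly shift the Left and Right panels in opposite directions with swept local offsets, gated by an IsOpen flag.
; With Break set, BeginPlay knocks the panels apart with slightly randomized tilts and destroys the box components, and Close does nothing.
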(event `OpenDoor`
  (if (not (`self.IsOpen`))
    (`self.Open`)
    (set `self.IsOpen` true)))

(event `self.ReceiveBeginPlay`
  (bind _right (`self.Right`))
  (bind _left (`self.Left`))
  (`|ExecutionSequence`
    (:`then_0`
      (if (`KismetMathLibrary.RandomBool`)
        (set `self.RandomRotation` 1)
        (else
          (set `self.RandomRotation` -1))))
    (:`then_1`
      (if (`self.Break`)
        (`SceneComponent.K2_AddLocalTransform` _right (`KismetMathLibrary.MakeTransform` (90.0 0.0 0.0) (`KismetMathLibrary.MakeRotator` (* (`KismetMathLibrary.RandomFloat`) (`self.RandomRotation`)) 4.0) (`SceneComponent.K2_GetComponentScale` _right)) true false)
        (`SceneComponent.K2_AddLocalTransform` _left (`KismetMathLibrary.MakeTransform` (-90.0 0.0 0.0) (`KismetMathLibrary.MakeRotator` 0.0 (* (`KismetMathLibrary.RandomFloat`) (`self.RandomRotation`))) (`SceneComponent.K2_GetComponentScale` _left)) true false)
        (`ActorComponent.K2_DestroyComponent` (`self.Box`))
        (`ActorComponent.K2_DestroyComponent` (`self.Box_0`))
        (`ActorComponent.K2_DestroyComponent` (`self.Box1`))))))

(event `self.Box_0.OnComponentBeginOverlap`
  (params (OverlappedComponent :type "PrimitiveComponent Object Reference") (OtherActor :type "Actor Object Reference") (OtherComp :type "PrimitiveComponent Object Reference") (OtherBodyIndex :type Integer) (bFromSweep :type Boolean) (SweepResult :type "HitResult Structure (by ref)"))
  (if (`self.IsOpen`)
    (set `self.IsOpen` false)
    (`self.Close`)))

(event `self.Box1.OnComponentBeginOverlap`
  (params (OverlappedComponent :type "PrimitiveComponent Object Reference") (OtherActor :type "Actor Object Reference") (OtherComp :type "PrimitiveComponent Object Reference") (OtherBodyIndex :type Integer) (bFromSweep :type Boolean) (SweepResult :type "HitResult Structure (by ref)"))
  (if (`self.IsOpen`)
    (set `self.IsOpen` false)
    (`self.Close`)))

(fn `Close`
  (bind _right (`self.Right`))
  (bind _left (`self.Left`))
  (if (not (`self.Break`))
    (`|ExecutionSequence`
      (:`then_0`
        (`SceneComponent.K2_AddLocalTransform` _right (`KismetMathLibrary.MakeTransform` (-100.0 0.0 0.0) (struct) (`SceneComponent.K2_GetComponentScale` _right)) true false))
      (:`then_1`
        (`SceneComponent.K2_AddLocalTransform` _left (`KismetMathLibrary.MakeTransform` (100.0 0.0 0.0) (struct) (`SceneComponent.K2_GetComponentScale` _left)) true false)))))

(fn `interact`
  (`parent.interact`)
  (`self.OpenDoor`))

(fn `Open`
  (bind _right (`self.Right`))
  (bind _left (`self.Left`))
  (`|ExecutionSequence`
    (:`then_0`
      (`SceneComponent.K2_AddLocalTransform` _right (`KismetMathLibrary.MakeTransform` (100.0 0.0 0.0) (struct) (`SceneComponent.K2_GetComponentScale` _right)) true false))
    (:`then_1`
      (`SceneComponent.K2_AddLocalTransform` _left (`KismetMathLibrary.MakeTransform` (-100.0 0.0 0.0) (struct) (`SceneComponent.K2_GetComponentScale` _left)) true false))))

(fn `UserConstructionScript`)