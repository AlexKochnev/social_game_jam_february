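; Blueprint function library with shared combat helpers for damage, death and status effects.
; DoDamage subtracts from a BP_ThirdPersonCharacter's CurrentHealth and calls DoDeath at zero, which empties the HUD health bar and destroys the actor.
; AddStatusEffect loops over requested effects and dispatches slowdown, periodic damage and delayed damage to handlers that are still empty.
; StatusEffectContusion, absent from that dispatch, stacks and starts a noise effect on the status manager.
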(fn `AddStatusEffect`
  (params (StatusEffectOfActor :type "/Game/Blueprints/StatusEffectManager Object Reference") (StatusEffect :type "Array of /Game/Blueprints/Enumerators/StatusEffectsEnumerator Enum"))
  (`/Engine/EditorBlueprintResources/StandardMacros.IsValid` StatusEffectOfActor
    (:`Is Valid`
      (for _array_element StatusEffect
        (switch `/Game/Blueprints/Enumerators/StatusEffectsEnumerator` _array_element
          (:`NewEnumerator0`
            (`self.StatusEffectSlowdown` StatusEffectOfActor))
          (:`NewEnumerator1`
            (`self.StatusEffectEverySecondsDamage` StatusEffectOfActor))
          (:`NewEnumerator2`
            (`self.StatusEffectDelayedDamage` StatusEffectOfActor)))))))

(fn `DoDamage`
  (params (DamagedActor :type "Actor Object Reference") (Damage :type "Float (double-precision)"))
  (`/Engine/EditorBlueprintResources/StandardMacros.IsValid` DamagedActor
    (:`Is Valid`
      (bind _asbp_third_person_character (cast `/Game/ThirdPerson/Blueprints/BP_ThirdPersonCharacter` DamagedActor)
        (:`then`
          (bind _output_get (set `/Game/ThirdPerson/Blueprints/BP_ThirdPersonCharacter.Current Health` (- (`/Game/ThirdPerson/Blueprints/BP_ThirdPersonCharacter.Current Health` _asbp_third_person_character) Damage) _asbp_third_person_character))
          (if (<= _output_get 0.0)
            (`self.DoDeath` _asbp_third_person_character)))
        (:`CastFailed`
          (`KismetSystemLibrary.PrintString` null "Cast failed: \"Cant Cast to BP_TPC in DoDamage\"" true true (struct :`R` 1.0 :`A` 1.0) 5.0))))))

(fn `DoDeath`
  (params (ActorToDeath :type "/Game/ThirdPerson/Blueprints/BP_ThirdPersonCharacter Object Reference"))
  (`/Engine/EditorBlueprintResources/StandardMacros.IsValid` ActorToDeath
    (:`Is Valid`
      (`ProgressBar.SetPercent` (`/Game/Blueprints/Hud/InGameHud.HealthBar` (`/Game/ThirdPerson/Blueprints/BP_ThirdPersonCharacter.InGameHud` ActorToDeath)) 0.0)
      (`Actor.K2_DestroyActor` ActorToDeath))))

(fn `StatusEffectContusion`
  (params (statusEffectManager :type "/Game/Blueprints/StatusEffectManager Object Reference"))
  (`/Game/Blueprints/StatusEffectManager.AddNoizeStack` statusEffectManager)
  (`/Game/Blueprints/StatusEffectManager.SetNoizeLevel` statusEffectManager)
  (`/Game/Blueprints/StatusEffectManager.StartNoize` statusEffectManager))

(fn `StatusEffectDelayedDamage`
  (params (statusEffectManager :type "/Game/Blueprints/StatusEffectManager Object Reference")))

(fn `StatusEffectEverySecondsDamage`
  (params (statusEffectManager :type "/Game/Blueprints/StatusEffectManager Object Reference")))

(fn `StatusEffectSlowdown`
  (params (statusEffectManager :type "/Game/Blueprints/StatusEffectManager Object Reference")))