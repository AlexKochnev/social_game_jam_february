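; StatusEffectManager manages a stack-based noise status effect that plays audio on its owner.
; AddNoizeStack raises the stack count up to a maximum, and SetNoizeLevel converts it to a ratio of that maximum.
; StartNoize uses that level as the ambient noise volume, activating the sound if needed.
; RundomNoizeSteps randomly switches between the owner's left and right sounds, while SlowdownSpeed is an empty stub.
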(fn `AddNoizeStack`
  (bind _noizestacks (`self.noizeStacks`))
  (if (< _noizestacks (`self.maxNoizeStacks`))
    (bind _result (`/Engine/EditorBlueprintResources/StandardMacros.IncrementInt` _noizestacks)
      (:`  `
        (set `self.noizeStacks` _result)))))

(fn `RundomNoizeSteps`
  (bind _owner (`self.Owner`))
  (bind _leftsound (`/Game/ThirdPerson/Blueprints/BP_ThirdPersonCharacter.LeftSound` _owner))
  (bind _rightsound (`/Game/ThirdPerson/Blueprints/BP_ThirdPersonCharacter.RightSound` _owner))
  (if (== (`KismetMathLibrary.RandomInteger` 2) 1)
    (`self.Activate` _rightsound false)
    (`self.Deactivate` _leftsound)
    (else
      (`self.Activate` _leftsound false)
      (`self.Deactivate` _rightsound))))

(fn `SetNoizeLevel`
  (set `self.NoizeLevel` (/ (`self.noizeStacks`) (`self.maxNoizeStacks`))))

(fn `SlowdownSpeed`)

(fn `StartNoize`
  (bind _ambientnoize (`/Game/ThirdPerson/Blueprints/BP_ThirdPersonCharacter.AmbientNoize` (`self.Owner`)))
  (if (`self.IsActive` _ambientnoize)
    (`AudioComponent.SetVolumeMultiplier` _ambientnoize (`self.NoizeLevel`))
    (else
      (`AudioComponent.SetVolumeMultiplier` _ambientnoize (`self.NoizeLevel`))
      (`self.Activate` _ambientnoize false))))